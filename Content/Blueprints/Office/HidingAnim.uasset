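; HidingAnim is an interactable hiding spot that lets the player hide and unhide.
; On BeginPlay it caches the Player_BP character.
; Each Interactable event flips a Hidden flag and calls the player's CallHide or CallUnhide, leaving the hiding logic to the player.
; A DoOnce on the hide branch updates the player HUD's objective title and text only on the first hide.
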(event EventInteractable
  (bind _player (Variables|Default|GetPlayer))
  (if (not (Variables|Default|GetHidden))
    (Default|CallHide _player)
    (Variables|Default|SetHidden true)
    (Utilities|FlowControl|DoOnce false
      (:Completed
        (Default|SetObjectiveText (Variables|/Game/Blueprints/Office/Player/Player_BP.Player_BP_C|GetHUD _player) (Variables|Default|GetObjectiveText) (Variables|Default|GetObjectiveTitle))))
    (else
      (Default|CallUnhide _player)
      (Variables|Default|SetHidden false))))

(event EventBeginPlay
  (bind _asplayer_bp (Utilities|Casting|CastToPlayer_BP (Game|GetPlayerCharacter 0)))
  (Variables|Default|SetPlayer _asplayer_bp))

(fn ConstructionScript)