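; ChairAnim is an interactable office chair that lets the player sit down and stand up.
; On BeginPlay it caches the player character as Player_BP, and each Interactable event toggles SatDown and calls the player's sit or stand function.
; The first sit also passes the chair's objective title and text to the player HUD through a DoOnce gate, so the objective is set only once.
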(event EventInteractable
  (bind _player (Variables|Default|GetPlayer))
  (if (not (Variables|Default|GetSatDown))
    (Default|CallSitDown _player)
    (Variables|Default|SetSatDown true)
    (Utilities|FlowControl|DoOnce false
      (:Completed
        (Default|SetObjectiveText (Variables|/Game/Blueprints/Office/Player/Player_BP.Player_BP_C|GetHUD _player) (Variables|Default|GetObjectiveText) (Variables|Default|GetObjectiveTitle))))
    (else
      (Default|CallStandup _player)
      (Variables|Default|SetSatDown false))))

(event EventBeginPlay
  (bind _asplayer_bp (Utilities|Casting|CastToPlayer_BP (Game|GetPlayerCharacter 0)))
  (Variables|Default|SetPlayer _asplayer_bp))

(fn ConstructionScript)