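; First-person player character for the office area, handling sprint, toggle crouch, interaction and HUD creation.
; Tick picks an idle, walk, sprint or falling camera shake from movement, and spring-interpolates the camera to smooth crouch height changes.
; Sprint scales walk speed from a base cached at BeginPlay, with events to cancel or resume it.
; Interact line-traces from the camera and messages the hit actor, while Space calls a stand-up event.
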(event Custom|CameraShake
  (bind _returnvalue (Game|GetPlayerController 0))
  ;[1 0 0] CameraShake
  (if (AI|Components|NavMovement|IsFalling (Variables|Character|GetCharacterMovement))
    (Game|Feedback|ClientStartCameraShake _returnvalue "/Game/Blueprints/Office/Player/CameraShake/Falling.Falling_C" 1.0 "CameraLocal" "0, 0, 0")
    (elif (<= (Math|Vector|VectorLength (Transformation|GetVelocity)) 0.0)
      (Game|Feedback|ClientStartCameraShake _returnvalue "/Game/Blueprints/Office/Player/CameraShake/Idle.Idle_C" 1.0 "CameraLocal" "0, 0, 0")
      (elif (>= (Math|Vector|VectorLength (Transformation|GetVelocity)) 3e+02)
        (Game|Feedback|ClientStartCameraShake _returnvalue "/Game/Blueprints/Office/Player/CameraShake/Sprint.Sprint_C" 1.0 "CameraLocal" "0, 0, 0")
        (else
          (Game|Feedback|ClientStartCameraShake _returnvalue "/Game/Blueprints/Office/Player/CameraShake/Walk.Walk_C" 1.0 "CameraLocal" "0, 0, 0"))))))

(event Custom|Sprint
  ;[1 0 0.8366 1 74] SprintSystem
  (Utilities|FlowControl|Delay 0.05)
  (if (Variables|Default|GetCanSprintBool?)
    (if (Variables|PlayerMovement|GetCrouch?)
      (Character|UnCrouch)
      (else
        (Variables|/Script/Engine.CharacterMovementComponent|SetMaxWalkSpeed (Variables|Character|GetCharacterMovement) (* (Variables|PlayerMovement|GetBaseSpeed) (Variables|PlayerMovement|GetSprintSpeedMultiplier)))
        (Variables|PlayerMovement|SetisSprinting? true)))))

(event Custom|SetCamPos
  ;[0.2789 1 0.2634 1 42] CrouchCamera
  (bind _output_get (Variables|PlayerMovement|SetCamPos (Variables|/Script/Engine.SceneComponent|GetRelativeLocation (Variables|Default|GetMainCamera))))
  (Variables|PlayerMovement|SetCurrentCamPos _output_get))

(event Custom|InterpTo
  (params (Delta :type Float%20%28double-precision%29))
  ;[0.2789 1 0.2634 1 42] CrouchCamera
  (bind _returnvalue (Class|KismetMathLibrary|VectorSpringInterp (Variables|PlayerMovement|GetCurrentCamPos) (Variables|PlayerMovement|GetCamPos) (Variables|PlayerMovement|GetCrouchSpring) 1.1e+03 0.8 Delta 7.0 0.9))
  (bind _output_get (Variables|PlayerMovement|SetCurrentCamPos _returnvalue))
  (Transformation|SetRelativeLocation (Variables|Default|GetMainCamera) _output_get false false))

(event Custom|VariableSet
  ;[1 1 1] SetVariables
  (Variables|PlayerMovement|SetBaseSpeed (* (Variables|PlayerMovement|GetSpeedMultiplier) (Variables|/Script/Engine.CharacterMovementComponent|GetMaxWalkSpeed (Variables|Character|GetCharacterMovement)))))

(event Custom|CanSprintAgain
  ;[1 0 0.8366 1 74] SprintSystem
  (if (Variables|PlayerMovement|GetSprintTemp)
    (Variables|/Script/Engine.CharacterMovementComponent|SetMaxWalkSpeed (Variables|Character|GetCharacterMovement) (* (Variables|PlayerMovement|GetBaseSpeed) (Variables|PlayerMovement|GetSprintSpeedMultiplier)))
    (Variables|PlayerMovement|SetisSprinting? true)))

(event Custom|CancelSprint
  ;[1 0 0.8366 1 74] SprintSystem
  (Variables|/Script/Engine.CharacterMovementComponent|SetMaxWalkSpeed (Variables|Character|GetCharacterMovement) (Variables|PlayerMovement|GetBaseSpeed))
  (Variables|PlayerMovement|SetisSprinting? false))

(event Input|EnhancedActionEvents|EnhancedInputActionIA_Crouch
  (params (ActionValue :type Boolean) (ElapsedSeconds :type Float%20%28double-precision%29) (TriggeredSeconds :type Float%20%28double-precision%29) (InputAction :type Input%20Action%20Object%20Reference :default "/Game/Blueprints/Office/Player/Inputs/IA_Crouch.IA_Crouch"))
  ;[0.2789 1 0.2634 1 42] CrouchCamera
  (CallFunction|CrouchF))

(event Input|EnhancedActionEvents|EnhancedInputActionIA_Interact
  (params (ActionValue :type Boolean) (ElapsedSeconds :type Float%20%28double-precision%29) (TriggeredSeconds :type Float%20%28double-precision%29) (InputAction :type Input%20Action%20Object%20Reference :default "/Game/Blueprints/Office/Player/Inputs/IA_Interact.IA_Interact"))
  (bind _maincamera (Variables|Default|GetMainCamera))
  (bind _returnvalue (Transformation|GetWorldLocation _maincamera))
  (bind (_outhit _returnvalue_2) (Collision|LineTraceByChannel _returnvalue (+ _returnvalue (* (Math|Vector|GetForwardVector _maincamera) (Variables|Default|GetInteractableRange))) "TraceTypeQuery1" false 0 "ForDuration" true "(R=1.000000,G=0.000000,B=0.000000,A=1.000000)" "(R=0.000000,G=1.000000,B=0.000000,A=1.000000)" 2.0))
  (if _returnvalue_2
    (Class|Interact|Interactable(Message) (.HitActor (Collision|BreakHitResult _outhit)))))

(event Input|EnhancedActionEvents|EnhancedInputActionIA_Sprint
  (params (ActionValue :type Boolean) (ElapsedSeconds :type Float%20%28double-precision%29) (TriggeredSeconds :type Float%20%28double-precision%29) (InputAction :type Input%20Action%20Object%20Reference :default "/Game/Blueprints/Office/Player/Inputs/IA_Sprint.IA_Sprint"))
  (bind _charactermovement (Variables|Character|GetCharacterMovement))
  ;[1 0 0.8366 1 74] SprintSystem
  (:Started
    (Variables|PlayerMovement|SetSprintTemp true)
    (if (Variables|Default|GetCanSprintBool?)
      (if (Variables|PlayerMovement|GetCrouch?)
        (Character|UnCrouch)
        (else
          (Variables|/Script/Engine.CharacterMovementComponent|SetMaxWalkSpeed _charactermovement (* (Variables|PlayerMovement|GetBaseSpeed) (Variables|PlayerMovement|GetSprintSpeedMultiplier)))
          (Variables|PlayerMovement|SetisSprinting? true)))))
  (:Completed
    (Variables|PlayerMovement|SetSprintTemp false)
    (Variables|/Script/Engine.CharacterMovementComponent|SetMaxWalkSpeed _charactermovement (Variables|PlayerMovement|GetBaseSpeed))
    (Variables|PlayerMovement|SetisSprinting? false)))

(event EventOnStartCrouch
  (params (HalfHeightAdjust :type Float%20%28single-precision%29) (ScaledHalfHeightAdjust :type Float%20%28single-precision%29))
  ;[0.2789 1 0.2634 1 42] CrouchCamera
  (if (not (AI|Components|NavMovement|IsFalling (Variables|Character|GetCharacterMovement)))
    (Variables|PlayerMovement|SetCurrentCamPos (+ (Variables|PlayerMovement|GetCamPos) (Math|Vector|MakeVector 0.0 0.0 ScaledHalfHeightAdjust)))))

(event EventTick
  (params (DeltaSeconds :type Float%20%28single-precision%29))
  ;[1 0 0.03269 1 74] EventTick
  (Utilities|FlowControl|Sequence
    (:then_0
      (CallFunction|CameraShake))
    (:then_1
      (CallFunction|Interpto DeltaSeconds))))

(event EventBeginPlay
  ;[1 0 0 1 48] EventBeginPlay
  (Utilities|FlowControl|Sequence
    (:then_0
      (CallFunction|VariableSet))
    (:then_1
      (CallFunction|CreateHUD))))

(event EventOnEndCrouch
  (params (HalfHeightAdjust :type Float%20%28single-precision%29) (ScaledHalfHeightAdjust :type Float%20%28single-precision%29))
  ;[0.2789 1 0.2634 1 42] CrouchCamera
  (if (not (AI|Components|NavMovement|IsFalling (Variables|Character|GetCharacterMovement)))
    (Variables|PlayerMovement|SetCurrentCamPos (- (Variables|PlayerMovement|GetCamPos) (Math|Vector|MakeVector 0.0 0.0 ScaledHalfHeightAdjust)))))

(event Input|KeyboardEvents|SpaceBar
  (params (Key :type Key%20Structure :default "None"))
  (:Pressed
    (Default|CallStandup)))

(event Custom|CreateHUD
  (Utilities|IsValid (Variables|Default|GetHUD)
    (:Is%20Valid
      _)
    (:Is%20Not%20Valid
      (bind _returnvalue (UserInterface|CreateWidget "/Game/Blueprints/Office/Player/Widget/HUD_WBP.HUD_WBP_C"))
      (Variables|Default|SetHUD _returnvalue)))
  (UserInterface|Viewport|AddtoViewport _returnvalue 0))

(fn ConstructionScript)

(fn CrouchF
  (if (Variables|PlayerMovement|GetCrouch?)
    (Character|UnCrouch)
    (Variables|PlayerMovement|SetCrouch? false)
    (else
      (Character|Crouch)
      (Variables|PlayerMovement|SetCrouch? true))))

(fn SetCamera
  (params (Camera :type Camera%20Component%20Object%20Reference)))

(fn SwitchCameraMain)